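; Trampoline interactable that bounces the third-person character when it overlaps the trampoline's box.
; On overlap, it checks for the exact ThirdPersonCharacter class, then launches the character with its horizontal velocity kept and vertical velocity inverted, overriding current velocity.
; It then plays a 2D trampoline sound and ends on a one-second delay with nothing after it.
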(event OnComponentBeginOverlap(Box)
  (params (OverlappedComponent :type Primitive%20Component%20Object%20Reference) (OtherActor :type Actor%20Object%20Reference) (OtherComp :type Primitive%20Component%20Object%20Reference) (OtherBodyIndex :type Integer) (bFromSweep :type Boolean) (SweepResult :type Hit%20Result%20Structure%20%28by%20ref%29))
  (bind _returnvalue (Transformation|GetVelocity OtherActor))
  (bind (_x _y _z) (Math|Vector|BreakVector _returnvalue))
  (if (== (Utilities|GetClass OtherActor) "/Game/BluePrints/ThirdPersonBP/Blueprints/ThirdPersonCharacter.ThirdPersonCharacter_C")
    (bind _asthird_person_character (Utilities|Casting|CastToThirdPersonCharacter OtherActor))
    (Character|LaunchCharacter _asthird_person_character (Math|Vector|MakeVector _x _y (* _z -1.0)) true true)
    (Audio|PlaySound2D "/Game/Sound/SFX-trampoline.SFX-trampoline" 1.0 1.0 0.0 0 0)
    (Utilities|FlowControl|Delay 1.0)))

(fn ConstructionScript)