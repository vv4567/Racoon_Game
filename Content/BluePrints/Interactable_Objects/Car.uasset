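; Car is an interactable hazard that launches the player's ThirdPersonCharacter upward when it enters the car's box trigger.
; The first hit also completes the "Get hit by Car" achievement through a DoOnce.
; That one-time sequence plays objective and raccoon sounds around a short delay, shows a Car widget, then clears all widgets from the viewport two seconds later.
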(event OnComponentBeginOverlap(Box)
  (params (OverlappedComponent :type Primitive%20Component%20Object%20Reference) (OtherActor :type Actor%20Object%20Reference) (OtherComp :type Primitive%20Component%20Object%20Reference) (OtherBodyIndex :type Integer) (bFromSweep :type Boolean) (SweepResult :type Hit%20Result%20Structure%20%28by%20ref%29))
  (bind _asthird_person_character (Utilities|Casting|CastToThirdPersonCharacter OtherActor))
  (Character|LaunchCharacter _asthird_person_character "0.000000,0.000000,1000.000000" false false)
  (Utilities|FlowControl|DoOnce false
    (:Completed
      ;[1 1 1] Achievment
      (Class|AchievementSubSystem|AddAchievementProgress (Subsystems|GetAchievementSubSystem) "Get hit by Car" 1e+02)
      (Audio|PlaySound2D "/Game/Sound/SFX-objective.SFX-objective" 1.0 1.0 0.0 0 0)
      (Utilities|FlowControl|Delay 1.0)
      (Audio|PlaySound2D "/Game/Sound/SFX-raccoon.SFX-raccoon" 1.0 1.0 0.0 0 0)
      (bind _returnvalue (UserInterface|CreateWidget "/Game/Objective_Widgets/Car.Car_C"))
      (UserInterface|Viewport|AddtoViewport _returnvalue 0)
      (Utilities|FlowControl|Delay 2.0)
      (Viewport|RemoveAllWidgets))))

(event EventBeginPlay)

(event Collision|EventActorBeginOverlap
  (params (OtherActor :type Actor%20Object%20Reference)))

(event EventTick
  (params (DeltaSeconds :type Float%20%28single-precision%29)))

(fn ConstructionScript)