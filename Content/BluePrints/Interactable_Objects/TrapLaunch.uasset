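; TrapLaunch is a one-shot bear trap that launches the player upward when stepped on.
; A Box overlap by a ThirdPersonCharacter passes a DoOnce, swaps the R mesh to the closed trap, plays a 2D trap sound and launches player 0 vertically.
; Disconnected leftover nodes for a car-hit sound, a "Get hit by Car" achievement and a widget popup never run.
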(event OnComponentBeginOverlap(Box)
  (params (OverlappedComponent :type Primitive%20Component%20Object%20Reference) (OtherActor :type Actor%20Object%20Reference) (OtherComp :type Primitive%20Component%20Object%20Reference) (OtherBodyIndex :type Integer) (bFromSweep :type Boolean) (SweepResult :type Hit%20Result%20Structure%20%28by%20ref%29))
  (Utilities|Casting|CastToThirdPersonCharacter OtherActor)
  (Utilities|FlowControl|DoOnce false
    (:Completed
      (Components|StaticMesh|SetStaticMesh (Variables|Default|Getr) "/Game/ArtAssets/Model/PhuocB/Closed_BearTrap.Closed_BearTrap")
      (Audio|PlaySound2D "/Game/Sound/SFX-trap.SFX-trap" 1.0 1.0 0.0 0 0)
      (Character|LaunchCharacter (Game|GetPlayerCharacter 0) "0.000000,0.000000,1000.000000" false false))))

(event EventBeginPlay)

(event Collision|EventActorBeginOverlap
  (params (OtherActor :type Actor%20Object%20Reference)))

(event EventTick
  (params (DeltaSeconds :type Float%20%28single-precision%29)))

(fn ConstructionScript)