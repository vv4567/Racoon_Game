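; Interactable rose pickup that the player collects by pressing Interact while standing in its trigger box.
; Box overlap enables input and, if the actor is the ThirdPersonCharacter, stores it and opens a gate; leaving disables input and closes the gate.
; Interacting through the open gate reveals the character's own Rose component, enables RoseBox collision on it, then destroys this actor.
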(event OnComponentBeginOverlap(Box)
  (params (OverlappedComponent :type Primitive%20Component%20Object%20Reference) (OtherActor :type Actor%20Object%20Reference) (OtherComp :type Primitive%20Component%20Object%20Reference) (OtherBodyIndex :type Integer) (bFromSweep :type Boolean) (SweepResult :type Hit%20Result%20Structure%20%28by%20ref%29))
  (Input|EnableInput (Game|GetPlayerController 0))
  (bind _asthird_person_character (Utilities|Casting|CastToThirdPersonCharacter OtherActor))
  (Utilities|FlowControl|Gate true) ; enters at Open
)

(event OnComponentEndOverlap(Box)
  (params (OverlappedComponent :type Primitive%20Component%20Object%20Reference) (OtherActor :type Actor%20Object%20Reference) (OtherComp :type Primitive%20Component%20Object%20Reference) (OtherBodyIndex :type Integer))
  (Input|DisableInput (Game|GetPlayerController 0))
  (Utilities|Casting|CastToThirdPersonCharacter OtherActor)
  (Utilities|FlowControl|Gate true) ; enters at Close
)

(event EventBeginPlay)

(event Collision|EventActorBeginOverlap
  (params (OtherActor :type Actor%20Object%20Reference)))

(event EventTick
  (params (DeltaSeconds :type Float%20%28single-precision%29)))

(event Input|ActionEvents|InputActionInteract
  (params (Key :type Key%20Structure :default "None"))
  (:Pressed
    (Utilities|FlowControl|Gate true
      (:Exit
        (Rendering|SetVisibility (Variables|/Game/BluePrints/ThirdPersonBP/Blueprints/ThirdPersonCharacter.ThirdPersonCharacter_C|Getrose (stale OnComponentBeginOverlap(Box) _asthird_person_character)) true false)
        (Collision|SetCollisionEnabled (Variables|/Game/BluePrints/ThirdPersonBP/Blueprints/ThirdPersonCharacter.ThirdPersonCharacter_C|GetRoseBox (stale OnComponentBeginOverlap(Box) _asthird_person_character)) "QueryAndPhysics")
        (Actor|DestroyActor)))))

(fn ConstructionScript)