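; Soccer goal interactable that reacts when a Ball enters it, awarding the "Goal" achievement.
; The Box overlap casts to Ball and passes a DoOnce, then adds achievement progress and plays an objective sound, followed by a delayed raccoon sound.
; A separate actor overlap event creates and animates the GOAL widget on any overlap, with no Ball check or once-only gate.
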(event OnComponentBeginOverlap(Box)
  (params (OverlappedComponent :type Primitive%20Component%20Object%20Reference) (OtherActor :type Actor%20Object%20Reference) (OtherComp :type Primitive%20Component%20Object%20Reference) (OtherBodyIndex :type Integer) (bFromSweep :type Boolean) (SweepResult :type Hit%20Result%20Structure%20%28by%20ref%29))
  (Utilities|Casting|CastToBall OtherActor)
  (Utilities|FlowControl|DoOnce false
    (:Completed
      ;[1 1 1] Achievment
      (Class|AchievementSubSystem|AddAchievementProgress (Subsystems|GetAchievementSubSystem) "Goal" 1e+02)
      (Audio|PlaySound2D "/Game/Sound/SFX-objective.SFX-objective" 1.0 1.0 0.0 0 0)
      (Utilities|FlowControl|Delay 1.0)
      (Audio|PlaySound2D "/Game/Sound/SFX-raccoon.SFX-raccoon" 1.0 1.0 0.0 0 0))))

(event EventBeginPlay)

(event Collision|EventActorBeginOverlap
  (params (OtherActor :type Actor%20Object%20Reference))
  (bind _returnvalue (UserInterface|CreateWidget "/Game/Objective_Widgets/GOAL.GOAL_C"))
  (UserInterface|Viewport|AddtoViewport _returnvalue 0)
  (UserInterface|Animation|PlayAnimation _returnvalue (Variables|/Game/Objective_Widgets/GOAL.GOAL_C|Getgoal _returnvalue) 0.0 1 "Forward" 1.0 false))

(event EventTick
  (params (DeltaSeconds :type Float%20%28single-precision%29)))

(fn ConstructionScript)