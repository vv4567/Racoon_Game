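; TrashBurger is an edible trash pickup that the player eats with the Interact input.
; Box overlap toggles input and, for ThirdPersonCharacter, opens or closes a gate that lets the press through.
; Eating plays a sound, destroys the burger, advances the "Eat Trash" achievement, raises jump velocity and calls RemoveTrash on the character.
; The walk speed adjustment adds zero, so only jumping improves.
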(event OnComponentBeginOverlap(Box)
  (params (OverlappedComponent :type Primitive%20Component%20Object%20Reference) (OtherActor :type Actor%20Object%20Reference) (OtherComp :type Primitive%20Component%20Object%20Reference) (OtherBodyIndex :type Integer) (bFromSweep :type Boolean) (SweepResult :type Hit%20Result%20Structure%20%28by%20ref%29))
  (Input|EnableInput (Game|GetPlayerController 0))
  (Utilities|Casting|CastToThirdPersonCharacter OtherActor)
  (Utilities|FlowControl|Gate true) ; enters at Open
)

(event OnComponentEndOverlap(Box)
  (params (OverlappedComponent :type Primitive%20Component%20Object%20Reference) (OtherActor :type Actor%20Object%20Reference) (OtherComp :type Primitive%20Component%20Object%20Reference) (OtherBodyIndex :type Integer))
  (Input|DisableInput (Game|GetPlayerController 0))
  (Utilities|Casting|CastToThirdPersonCharacter OtherActor)
  (Utilities|FlowControl|Gate true) ; enters at Close
)

(event EventBeginPlay)

(event Collision|EventActorBeginOverlap
  (params (OtherActor :type Actor%20Object%20Reference)))

(event EventTick
  (params (DeltaSeconds :type Float%20%28single-precision%29)))

(event Input|ActionEvents|InputActionInteract
  (params (Key :type Key%20Structure :default "None"))
  (:Pressed
    (Utilities|FlowControl|Gate true
      (:Exit
        (bind _asthird_person_character (Utilities|Casting|CastToThirdPersonCharacter (Game|GetPlayerCharacter 0)))
        (Audio|PlaySound2D "/Game/Sound/SFX-eating.SFX-eating" 1.0 1.0 0.0 0 0)
        (Utilities|FlowControl|Sequence
          (:then_0
            ;[1 1 1] Walk speed
            (Variables|/Script/Engine.CharacterMovementComponent|SetMaxWalkSpeed (Variables|/Script/Engine.Character|GetCharacterMovement _asthird_person_character) (+ (Variables|/Script/Engine.CharacterMovementComponent|GetMaxWalkSpeed (Variables|/Script/Engine.Character|GetCharacterMovement _asthird_person_character)) 0.0))
            ;[1 1 1] Achievment
            (Actor|DestroyActor)
            (Class|AchievementSubSystem|AddAchievementProgress (Subsystems|GetAchievementSubSystem) "Eat Trash" 1.0)
            (Development|PrintString "Stat Increase!"))
          (:then_1
            ;[1 1 1] Jump Height
            (Variables|/Script/Engine.CharacterMovementComponent|SetJumpZVelocity (Variables|/Script/Engine.Character|GetCharacterMovement _asthird_person_character) (+ (Variables|/Script/Engine.CharacterMovementComponent|GetJumpZVelocity (Variables|/Script/Engine.Character|GetCharacterMovement _asthird_person_character)) 15.0)))
          (:then_2
            (Default|RemoveTrash _asthird_person_character)))))))

(fn ConstructionScript)